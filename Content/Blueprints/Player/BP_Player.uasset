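; Player character Blueprint for a third-person rifle shooter, creating health bar, magazine and crosshair widgets.
; A looping timer drives automatic fire, spawning tracers and applying point damage via line traces from the camera when aiming, otherwise from the muzzle.
; Aiming drives ABP_Character and a switchable over-shoulder camera; reload refills after a delay.
; PointDamage reduces HP, ragdolling and opening GameOver at zero, while AnyDamage updates a separate Health variable.
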(event Custom|On%20Fire
  (bind _weapon (Variables|Default|GetWeapon))
  (bind _followcamera (Variables|Default|GetFollowCamera))
  (bind _weapon_2 (Variables|Default|GetWeapon))
  (bind _weapon_3 (Variables|Default|GetWeapon))
  (bind _returnvalue (Transformation|GetSocketTransform _weapon_3 "MuzzleFlash" "RTS_World"))
  (bind _returnvalue_2 (Transformation|GetSocketTransform _weapon "MuzzleFlash" "RTS_World"))
  (bind _returnvalue_3 (Transformation|GetWorldLocation _followcamera))
  (bind _returnvalue_4 (Transformation|GetSocketTransform _weapon_2 "MuzzleFlash" "RTS_World"))
  ;[1 1 1] 射撃アニメーションをループ再生
  (Animation|Montage|PlayMontage (Variables|Character|GetMesh) "/Game/Animations/TPSAnimation/Game/Characters/Heroes/Mannequin/Animations/Actions/MM_Rifle_Fire_Montage.MM_Rifle_Fire_Montage" ; 射撃アニメーションを再生
    (:then
      ;[1 1 1] マガジンの残弾数によって射撃できるか？どうかを分岐させる
      (if (< 0 (Variables|Default|Getmagazine))
        (Variables|Default|Setmagazine (- (Variables|Default|Getmagazine) 1))
        (Effects|SpawnEmitteratLocation "/Game/MilitaryWeapSilver/FX/P_AssaultRifle_MuzzleFlash.P_AssaultRifle_MuzzleFlash" (.location _returnvalue_4) (.rotation _returnvalue_4)) ; マズルフラッシュのエフェクトを出す
        (Audio|PlaySoundatLocation "/Game/MilitaryWeapSilver/Sound/Rifle/Cues/RifleA_Fire_Cue.RifleA_Fire_Cue" (.location _returnvalue_4) "0, 0, 0" 1.0 1.0 0.0 0 0 0 0) ; 銃声音を再生する
        (if (Variables|Default|GetisLocalAiming) ; エイム中かどうか？
          ;[1 1 1 1 30] カメラからレイを出して攻撃する
          (bind (_outhit _returnvalue_5) (Collision|LineTraceByChannel _returnvalue_3 (+ _returnvalue_3 (* (Math|Vector|GetForwardVector (Transformation|GetWorldRotation _followcamera)) 5e+03)) "TraceTypeQuery1" false 0 "ForDuration" true "(R=1.000000,G=0.000000,B=0.039356,A=1.000000)")) ; StartからEndに向かってレイを飛ばすノード
          (Game|SpawnActorfromClass "/Game/Blueprints/Player/BP_RilfeTracer.BP_RilfeTracer_C" (Math|Transform|MakeTransform (.location _returnvalue) (Math|Rotator|FindLookatRotation (.location _returnvalue) (.TraceEnd (Collision|BreakHitResult _outhit))) (.scale _returnvalue)) "AlwaysSpawn" 0 0) ; 銃弾の軌跡のアクターを生成する
          (if _returnvalue_5
            (Game|Damage|ApplyPointDamage (.HitActor (Collision|BreakHitResult _outhit)) 1e+01 (.TraceStart (Collision|BreakHitResult _outhit)) _outhit) ; アクターにダメージを与えるノード
          )
          (else
            ;[1 1 1 1 30] 銃口からレイを出して攻撃する
            (bind (_outhit_2 _returnvalue_6) (Collision|LineTraceByChannel (.location _returnvalue_2) (+ (.location _returnvalue_2) (* (Math|Vector|GetForwardVector (.rotation _returnvalue_2)) 5e+03)) "TraceTypeQuery1" false 0 "ForDuration" true "(R=1.000000,G=0.163331,B=0.000000,A=1.000000)")) ; StartからEndに向かってレイを飛ばすノード
            (Game|SpawnActorfromClass "/Game/Blueprints/Player/BP_RilfeTracer.BP_RilfeTracer_C" (Transformation|GetSocketTransform (Variables|Default|GetWeapon) "MuzzleFlash" "RTS_World") "AlwaysSpawn" 0 0) ; 銃弾の軌跡のアクターを生成する
            (if _returnvalue_6
              (Game|Damage|ApplyPointDamage (.HitActor (Collision|BreakHitResult _outhit_2)) 1e+01 (.TraceStart (Collision|BreakHitResult _outhit_2)) _outhit_2) ; アクターにダメージを与えるノード
            )))
        (else
          ;[1 1 1] 射撃アニメーションのループ再生を終了させる
          (Utilities|Time|ClearandInvalidateTimerbyHandle (Variables|Default|GetFireTimer)))))))

(event EventBeginPlay
  ;[1 1 1] クロスヘアUIを作成する
  (bind _returnvalue (UserInterface|CreateWidget "/Game/UI/UI_Crosshair.UI_Crosshair_C"))
  (Variables|Default|SetCrosshairWidget _returnvalue)
  ;[1 1 1] 2層式HPゲージを作成する
  (bind _returnvalue_2 (UserInterface|CreateWidget "/Game/UI/UI_2LayersHealthBar.UI_2LayersHealthBar_C"))
  (bind _output_get (Variables|Default|SetHealthBar _returnvalue_2))
  (UserInterface|Viewport|AddtoViewport _output_get 0)
  ;[1 1 1] マガジンのUIを作成
  (bind _returnvalue_3 (UserInterface|CreateWidget "/Game/UI/UI_Magazine.UI_Magazine_C"))
  (bind _output_get_2 (Variables|Default|SetMagazineUI _returnvalue_3))
  (UserInterface|Viewport|AddtoViewport _output_get_2 0))

(event Collision|EventActorBeginOverlap
  (params (OtherActor :type Actor%20Object%20Reference)))

(event EventTick
  (params (DeltaSeconds :type Float%20%28single-precision%29)))

(event Game|Damage|EventPointDamage
  (params (Damage :type Float%20%28single-precision%29) (DamageType :type Damage%20Type%20Object%20Reference) (HitLocation :type Vector :default "0, 0, 0") (HitNormal :type Vector :default "0, 0, 0") (HitComponent :type Primitive%20Component%20Object%20Reference) (BoneName :type Name :default "None") (ShotFromDirection :type Vector :default "0, 0, 0") (InstigatedBy :type Controller%20Object%20Reference) (DamageCauser :type Actor%20Object%20Reference) (HitInfo :type Hit%20Result%20Structure%20%28by%20ref%29))
  ;[1 1 1] ダメージを受ける処理
  (bind _output_get (Variables|Default|SetHP (- (Variables|Default|GetHP) Damage)))
  (Default|UpdateHealthBar (Variables|Default|GetHealthBar) (/ _output_get (Variables|Default|GetMaxHP)))
  (Development|PrintString (Utilities|String|ToString(Float) _output_get) true true "(R=1.000000,G=0.434760,B=0.000000,A=1.000000)" 5.0)
  (if (<= _output_get 0.0)
    (Development|PrintString "Dead" true true "(R=1.000000,G=0.000000,B=0.058791,A=1.000000)" 1e+01)
    ;[1 1 1] 2層式HPゲージのUIを消す、そうしないとプレイヤーキャラクターが見つけられずエラーになる
    (Widget|RemovefromParent (Variables|Default|GetHealthBar))
    ;[1 1 1] マガジンUIを消す
    (Widget|RemovefromParent (Variables|Default|GetMagazineUI))
    ;[1 1 1] 物理シミュレーションでキャラクターが倒れる処理
    (Class|SkeletalMeshComponent|SetAllBodiesSimulatePhysics (Variables|Character|GetMesh) true)
    (Collision|SetCollisionEnabled (Variables|Character|GetMesh) "PhysicsOnly")
    (Input|DisableInput (Game|GetPlayerController 0)) ; キャラクターの入力を受け付けなくするノード
    (Utilities|FlowControl|Delay 3.0)
    (Game|OpenLevel(byObjectReference) "/Game/Maps/GameOver.GameOver")))

(event Game|Damage|EventAnyDamage
  (params (Damage :type Float%20%28single-precision%29) (DamageType :type Damage%20Type%20Object%20Reference) (InstigatedBy :type Controller%20Object%20Reference) (DamageCauser :type Actor%20Object%20Reference))
  (bind _output_get (Variables|Default|SetHealth (- (Variables|Default|GetHealth) Damage)))
  (Default|UpdateHealthBar (Variables|Default|GetHealthBar) (/ _output_get (Variables|Default|GetMaxHealth))))

(event Input|ActionEvents|InputActionFire
  (params (Key :type Key%20Structure :default "None"))
  (bind _weapon (Variables|Default|GetWeapon))
  (bind _followcamera (Variables|Default|GetFollowCamera))
  (bind _weapon_2 (Variables|Default|GetWeapon))
  (bind _weapon_3 (Variables|Default|GetWeapon))
  (bind _returnvalue (Transformation|GetSocketTransform _weapon_3 "MuzzleFlash" "RTS_World"))
  (bind _returnvalue_2 (Transformation|GetSocketTransform _weapon "MuzzleFlash" "RTS_World"))
  (bind _returnvalue_3 (Transformation|GetWorldLocation _followcamera))
  (bind _returnvalue_4 (Transformation|GetSocketTransform _weapon_2 "MuzzleFlash" "RTS_World"))
  (:Pressed
    ;[1 1 1] 射撃アニメーションをループ再生
    (Animation|Montage|PlayMontage (Variables|Character|GetMesh) "/Game/Animations/TPSAnimation/Game/Characters/Heroes/Mannequin/Animations/Actions/MM_Rifle_Fire_Montage.MM_Rifle_Fire_Montage" ; 射撃アニメーションを再生
      (:then
        (bind _returnvalue_5 (Utilities|Time|SetTimerbyEvent (delegate Custom|On%20Fire) 0.1 true)) ; 0.1秒後にEventが実行される
        (Variables|Default|SetFireTimer _returnvalue_5)
        ;[1 1 1] マガジンの残弾数によって射撃できるか？どうかを分岐させる
        (if (< 0 (Variables|Default|Getmagazine))
          (Variables|Default|Setmagazine (- (Variables|Default|Getmagazine) 1))
          (Effects|SpawnEmitteratLocation "/Game/MilitaryWeapSilver/FX/P_AssaultRifle_MuzzleFlash.P_AssaultRifle_MuzzleFlash" (.location _returnvalue_4) (.rotation _returnvalue_4)) ; マズルフラッシュのエフェクトを出す
          (Audio|PlaySoundatLocation "/Game/MilitaryWeapSilver/Sound/Rifle/Cues/RifleA_Fire_Cue.RifleA_Fire_Cue" (.location _returnvalue_4) "0, 0, 0" 1.0 1.0 0.0 0 0 0 0) ; 銃声音を再生する
          (if (Variables|Default|GetisLocalAiming) ; エイム中かどうか？
            ;[1 1 1 1 30] カメラからレイを出して攻撃する
            (bind (_outhit _returnvalue_6) (Collision|LineTraceByChannel _returnvalue_3 (+ _returnvalue_3 (* (Math|Vector|GetForwardVector (Transformation|GetWorldRotation _followcamera)) 5e+03)) "TraceTypeQuery1" false 0 "ForDuration" true "(R=1.000000,G=0.000000,B=0.039356,A=1.000000)")) ; StartからEndに向かってレイを飛ばすノード
            (Game|SpawnActorfromClass "/Game/Blueprints/Player/BP_RilfeTracer.BP_RilfeTracer_C" (Math|Transform|MakeTransform (.location _returnvalue) (Math|Rotator|FindLookatRotation (.location _returnvalue) (.TraceEnd (Collision|BreakHitResult _outhit))) (.scale _returnvalue)) "AlwaysSpawn" 0 0) ; 銃弾の軌跡のアクターを生成する
            (if _returnvalue_6
              (Game|Damage|ApplyPointDamage (.HitActor (Collision|BreakHitResult _outhit)) 1e+01 (.TraceStart (Collision|BreakHitResult _outhit)) _outhit) ; アクターにダメージを与えるノード
            )
            (else
              ;[1 1 1 1 30] 銃口からレイを出して攻撃する
              (bind (_outhit_2 _returnvalue_7) (Collision|LineTraceByChannel (.location _returnvalue_2) (+ (.location _returnvalue_2) (* (Math|Vector|GetForwardVector (.rotation _returnvalue_2)) 5e+03)) "TraceTypeQuery1" false 0 "ForDuration" true "(R=1.000000,G=0.163331,B=0.000000,A=1.000000)")) ; StartからEndに向かってレイを飛ばすノード
              (Game|SpawnActorfromClass "/Game/Blueprints/Player/BP_RilfeTracer.BP_RilfeTracer_C" (Transformation|GetSocketTransform (Variables|Default|GetWeapon) "MuzzleFlash" "RTS_World") "AlwaysSpawn" 0 0) ; 銃弾の軌跡のアクターを生成する
              (if _returnvalue_7
                (Game|Damage|ApplyPointDamage (.HitActor (Collision|BreakHitResult _outhit_2)) 1e+01 (.TraceStart (Collision|BreakHitResult _outhit_2)) _outhit_2) ; アクターにダメージを与えるノード
              )))
          (else
            ;[1 1 1] 射撃アニメーションのループ再生を終了させる
            (Utilities|Time|ClearandInvalidateTimerbyHandle (Variables|Default|GetFireTimer)))))))
  (:Released
    ;[1 1 1] 射撃アニメーションのループ再生を終了させる
    (Utilities|Time|ClearandInvalidateTimerbyHandle (Variables|Default|GetFireTimer))))

(event Input|ActionEvents|InputActionAiming
  (params (Key :type Key%20Structure :default "None"))
  (bind _mesh (Variables|Character|GetMesh))
  (bind _crosshairwidget (Variables|Default|GetCrosshairWidget))
  (bind _returnvalue (Components|SkeletalMesh|GetAnimInstance _mesh))
  (:Pressed
    (Variables|Default|SetisLocalAiming true) ; エイムしている
    (bind _asabp_character (Utilities|Casting|CastToABP_Character _returnvalue)) ; ABP_Characterにアクセスするためのノード
    (Variables|/Game/Animations/ABP_Character.ABP_Character_C|SetIsAiming? _asabp_character true) ; エイム用のアニメーションをON
    ;[1 1 1] 新しい肩越しカメラシステム
    (if (Variables|Default|GetCrosshairViewpoint)
      (CallFunction|SetViewpoint "300.000000,50.000000,70.000000" "0, 0, 0" false true) ; 右肩越しカメラ（Xが奥、Yが横、Zが縦）
      ;[1 1 1] クロスヘアを表示
      (UserInterface|Viewport|AddtoViewport _crosshairwidget 0)
      (else
        (CallFunction|SetViewpoint "300.000000,-50.000000,70.000000" "0, 0, 0" false true) ; 左肩越しカメラ（Xが奥、Yが横、Zが縦）
        (UserInterface|Viewport|AddtoViewport _crosshairwidget 0))))
  (:Released
    (Variables|Default|SetisLocalAiming false) ; エイムしていない
    (bind _asabp_character_2 (Utilities|Casting|CastToABP_Character _returnvalue))
    (Variables|/Game/Animations/ABP_Character.ABP_Character_C|SetIsAiming? _asabp_character_2 false) ; エイム用のアニメーションをOFF
    (CallFunction|SetViewpoint "0, 0, 0" "0, 0, 0" true false) ; 通常カメラ
    ;[1 1 1] クロスヘアを削除
    (Widget|RemovefromParent (Variables|Default|GetCrosshairWidget))))

(event Input|ActionEvents|InputActionToggleViewPoint
  (params (Key :type Key%20Structure :default "None"))
  (:Pressed
    (Utilities|FlowControl|FlipFlop ; Vキーを押すたびに視点が切り替わる
      (:A
        (Variables|Default|SetCrosshairViewpoint true) ; 肩越し右肩視点カメラ
      )
      (:B
        (Variables|Default|SetCrosshairViewpoint false) ; 肩越し左肩視点カメラ
      ))))

(event Input|ActionEvents|InputActionReload
  (params (Key :type Key%20Structure :default "None"))
  (:Pressed
    ;[1 1 1] リロードシステム
    (Audio|PlaySoundatLocation "/Game/SE/Reload.Reload" (.location (Transformation|GetSocketTransform (Variables|Default|GetWeapon) "MuzzleFlash" "RTS_World")) "0, 0, 0" 1.0 1.0 0.0 0 0 0 0) ; リロード音を再生する
    (Utilities|FlowControl|Delay 3.0)
    (Variables|Default|Setmagazine (Variables|Default|GetmagazineMax)) ; マガジンの最大数をマガジンに入れる
  ))

(event Input|KeyboardEvents|P
  (params (Key :type Key%20Structure :default "None"))
  (:Pressed
    (Game|Damage|ApplyDamage self 2e+01 0 0)))

(fn ConstructionScript)

(fn SetViewpoint
  (params (NewLocation :type Vector) (NewRotation :type Rotator) (Orient%20Rotation%20to%20Movement :type Boolean) (Use%20Controller%20Rotation%20Yaw :type Boolean))
  (Transformation|SetRelativeLocationAndRotation (Variables|Default|GetFollowCamera) NewLocation NewRotation false false)
  (Variables|/Script/Engine.CharacterMovementComponent|SetbOrientRotationToMovement (Variables|Character|GetCharacterMovement) Orient%20Rotation%20to%20Movement)
  (Variables|Default|SetbUseControllerRotationYaw Use%20Controller%20Rotation%20Yaw))