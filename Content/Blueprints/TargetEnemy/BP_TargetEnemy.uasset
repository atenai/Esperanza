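; BP_TargetEnemy is a damageable target enemy that ragdolls when killed.
; On receiving point damage it subtracts the amount from Health and prints the remaining value on screen.
; At zero or below it prints "Dead" and switches its mesh to physics simulation with physics-only collision, leaving the body in the world.
; Nodes for timed or immediate actor removal are present but unconnected.
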(event EventBeginPlay)

(event Collision|EventActorBeginOverlap
  (params (OtherActor :type Actor%20Object%20Reference)))

(event EventTick
  (params (DeltaSeconds :type Float%20%28single-precision%29)))

(event Game|Damage|EventPointDamage
  (params (Damage :type Float%20%28single-precision%29) (DamageType :type Damage%20Type%20Object%20Reference) (HitLocation :type Vector :default "0, 0, 0") (HitNormal :type Vector :default "0, 0, 0") (HitComponent :type Primitive%20Component%20Object%20Reference) (BoneName :type Name :default "None") (ShotFromDirection :type Vector :default "0, 0, 0") (InstigatedBy :type Controller%20Object%20Reference) (DamageCauser :type Actor%20Object%20Reference) (HitInfo :type Hit%20Result%20Structure%20%28by%20ref%29))
  ;[1 1 1] ダメージを受ける処理
  (bind _output_get (Variables|Default|SetHealth (- (Variables|Default|GetHealth) Damage)))
  (Development|PrintString (Utilities|String|ToString(Float) _output_get) true true "(R=1.000000,G=0.434760,B=0.000000,A=1.000000)" 5.0)
  (if (<= _output_get 0.0)
    (Development|PrintString "Dead" true true "(R=1.000000,G=0.000000,B=0.058791,A=1.000000)" 1e+01)
    ;[1 1 1] 物理シミュレーションでキャラクターが倒れる処理
    (Class|SkeletalMeshComponent|SetAllBodiesSimulatePhysics (Variables|Character|GetMesh) true)
    (Collision|SetCollisionEnabled (Variables|Character|GetMesh) "PhysicsOnly")))

(fn ConstructionScript)