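; Player Blueprint that handles automatic rifle fire feedback, with no projectile, trace or damage logic.
; Pressing Fire plays the fire montage on the mesh, starts a looping timer, and spawns muzzle flash and gunshot sound at the weapon's MuzzleFlash socket.
; The timer's OnFire event replays the montage and shares the same effects chain until releasing Fire clears the timer.
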(event Custom|On%20Fire
  (bind _weapon (Variables|Default|GetWeapon))
  (bind _returnvalue (Transformation|GetSocketTransform _weapon "MuzzleFlash" "RTS_World"))
  (Animation|Montage|PlayMontage (Variables|Character|GetMesh) "/Game/Animations/TPSAnimation/Game/Characters/Heroes/Mannequin/Animations/Actions/MM_Rifle_Fire_Montage.MM_Rifle_Fire_Montage" ; 射撃アニメーションを再生
    (:then
      (Effects|SpawnEmitteratLocation "/Game/MilitaryWeapSilver/FX/P_AssaultRifle_MuzzleFlash.P_AssaultRifle_MuzzleFlash" (.location _returnvalue) (.rotation _returnvalue)) ; マズルフラッシュのエフェクトを出す
      (Audio|PlaySoundatLocation "/Game/MilitaryWeapSilver/Sound/Rifle/Cues/RifleA_Fire_Cue.RifleA_Fire_Cue" (.location _returnvalue) "0, 0, 0" 1.0 1.0 0.0 0 0 0 0) ; 銃声音を再生する
    )))

(event EventBeginPlay)

(event Collision|EventActorBeginOverlap
  (params (OtherActor :type Actor%20Object%20Reference)))

(event EventTick
  (params (DeltaSeconds :type Float%20%28single-precision%29)))

(event Input|ActionEvents|InputActionFire
  (params (Key :type Key%20Structure :default "None"))
  (bind _weapon (Variables|Default|GetWeapon))
  (bind _returnvalue (Transformation|GetSocketTransform _weapon "MuzzleFlash" "RTS_World"))
  (:Pressed
    (Animation|Montage|PlayMontage (Variables|Character|GetMesh) "/Game/Animations/TPSAnimation/Game/Characters/Heroes/Mannequin/Animations/Actions/MM_Rifle_Fire_Montage.MM_Rifle_Fire_Montage" ; 射撃アニメーションを再生
      (:then
        (bind _returnvalue_2 (Utilities|Time|SetTimerbyEvent (delegate Custom|On%20Fire) 0.1 true)) ; 0.1秒後にEventが実行される
        (Variables|Default|SetFireTimer _returnvalue_2)
        (Effects|SpawnEmitteratLocation "/Game/MilitaryWeapSilver/FX/P_AssaultRifle_MuzzleFlash.P_AssaultRifle_MuzzleFlash" (.location _returnvalue) (.rotation _returnvalue)) ; マズルフラッシュのエフェクトを出す
        (Audio|PlaySoundatLocation "/Game/MilitaryWeapSilver/Sound/Rifle/Cues/RifleA_Fire_Cue.RifleA_Fire_Cue" (.location _returnvalue) "0, 0, 0" 1.0 1.0 0.0 0 0 0 0) ; 銃声音を再生する
      )))
  (:Released
    (Utilities|Time|ClearandInvalidateTimerbyHandle (Variables|Default|GetFireTimer))))

(fn ConstructionScript)