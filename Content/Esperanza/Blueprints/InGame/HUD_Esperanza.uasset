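; In-game HUD for Esperanza that owns the pause menu and exposes events for pausing, level changes and quitting.
; BeginPlay creates the pause widget collapsed in the viewport.
; DispPause_Event toggles its visibility, game pause, mouse cursor and UI-only or game-only input, while separate events open a named level or quit.
; Magazine and two-layer health bar creation remains in the graph but is unconnected, so never runs.
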(event Custom|DispPause_Event
  (params (IsPause :type Boolean))
  (bind _returnvalue (Game|Player|GetOwningPlayerController))
  (if IsPause
    ;[1 1 1] ポーズメニューをUIモードで表示する
    (Utilities|FlowControl|Sequence
      (:then_0
        (bind _pausemenuwidget (Variables|Default|GetPauseMenuWidget)
          (:then
            (Widget|SetVisibility _pausemenuwidget "Visible") ; VisibleでUIを表示
            (Input|SetInputModeUIOnly (Game|Player|GetOwningPlayerController) _pausemenuwidget "DoNotLock" false))
          (:else)))
      (:then_1
        (Game|SetGamePaused true)
        (Variables|/Script/Engine.PlayerController|SetbShowMouseCursor (Game|Player|GetOwningPlayerController) true)))
    (else
      ;[1 1 1] ポーズ状態を解除する
      (Game|SetGamePaused false)
      (Variables|/Script/Engine.PlayerController|SetbShowMouseCursor _returnvalue false)
      (Input|SetInputModeGameOnly _returnvalue false)
      (bind _pausemenuwidget_2 (Variables|Default|GetPauseMenuWidget)
        (:then
          (Widget|SetVisibility _pausemenuwidget_2 "Collapsed"))
        (:else)))))

(event Custom|OpenLevel_Event
  (params (LevelName :type Name))
  (Game|OpenLevel(byName) LevelName))

(event Custom|QuitGame_Event
  (Game|QuitGame (Game|Player|GetOwningPlayerController) "Quit" false))

(event EventBeginPlay
  (Utilities|FlowControl|Sequence
    (:then_0
      ;[1 1 1] ポーズメニューを非表示で生成する
      (bind _returnvalue (UserInterface|CreateWidget "/Game/Esperanza/UI/UI_Pause.UI_Pause_C" (Game|Player|GetOwningPlayerController)))
      (bind _output_get (Variables|Default|SetPauseMenuWidget _returnvalue))
      (Widget|SetVisibility _output_get "Collapsed") ; CollapsedでUIを畳む
      (UserInterface|Viewport|AddtoViewport _output_get 0))))

(event EventTick
  (params (DeltaSeconds :type Float%20%28single-precision%29)))

(fn ConstructionScript)