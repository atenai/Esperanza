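; BP_AIEnemy is a rifle-wielding enemy that takes point damage and ragdolls on death.
; Fire, while alive, plays a montage with muzzle flash, sound and a tracer actor from the weapon's MuzzleFlash socket.
; A debug-drawn Visibility line trace from that socket applies point damage to whatever it hits.
; PointDamage lowers and prints Health; at zero it clears Alive, enables mesh physics and destroys the capsule.
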(event Custom|Fire
  (bind _weapon (Variables|Default|GetWeapon))
  (bind _weapon_2 (Variables|Default|GetWeapon))
  (bind _returnvalue (Transformation|GetSocketTransform _weapon_2 "MuzzleFlash" "RTS_World"))
  (bind _returnvalue_2 (Transformation|GetSocketTransform _weapon "MuzzleFlash" "RTS_World"))
  (if (Variables|Default|GetAlive?)
    (Animation|Montage|PlayMontage (Variables|Character|GetMesh) "/Game/Esperanza/Animations/TPSAnimation/Game/Characters/Heroes/Mannequin/Animations/Actions/MM_Rifle_Fire_Montage.MM_Rifle_Fire_Montage" ; 射撃アニメーションを再生
      (:then
        (Effects|SpawnEmitteratLocation "/Game/MilitaryWeapSilver/FX/P_AssaultRifle_MuzzleFlash.P_AssaultRifle_MuzzleFlash" (.location _returnvalue_2) (.rotation _returnvalue_2)) ; マズルフラッシュのエフェクトを出す
        (Audio|PlaySoundatLocation "/Game/MilitaryWeapSilver/Sound/Rifle/Cues/RifleA_Fire_Cue.RifleA_Fire_Cue" (.location _returnvalue_2) "0, 0, 0" 1.0 1.0 0.0 0 0 0 0) ; 銃声音を再生する
        ;[1 1 1 1 30] 銃口からレイを出して攻撃する
        (bind (_outhit _returnvalue_3) (Collision|LineTraceByChannel (.location _returnvalue) (+ (.location _returnvalue) (* (Math|Vector|GetForwardVector (.rotation _returnvalue)) 5e+03)) "TraceTypeQuery1" false 0 "ForDuration" true "(R=1.000000,G=0.163331,B=0.000000,A=1.000000)")) ; StartからEndに向かってレイを飛ばすノード
        (Game|SpawnActorfromClass "/Game/Esperanza/Blueprints/Player/BP_RilfeTracer.BP_RilfeTracer_C" (Transformation|GetSocketTransform (Variables|Default|GetWeapon) "MuzzleFlash" "RTS_World") "AlwaysSpawn" 0 0) ; 銃弾の軌跡のアクターを生成する
        (if _returnvalue_3
          (Game|Damage|ApplyPointDamage (.HitActor (Collision|BreakHitResult _outhit)) 1e+01 (.TraceStart (Collision|BreakHitResult _outhit)) _outhit) ; アクターにダメージを与えるノード
        )))))

(event Game|Damage|EventPointDamage
  (params (Damage :type Float%20%28single-precision%29) (DamageType :type Damage%20Type%20Object%20Reference) (HitLocation :type Vector :default "0, 0, 0") (HitNormal :type Vector :default "0, 0, 0") (HitComponent :type Primitive%20Component%20Object%20Reference) (BoneName :type Name :default "None") (ShotFromDirection :type Vector :default "0, 0, 0") (InstigatedBy :type Controller%20Object%20Reference) (DamageCauser :type Actor%20Object%20Reference) (HitInfo :type Hit%20Result%20Structure%20%28by%20ref%29))
  ;[1 1 1] ダメージを受ける処理
  (bind _output_get (Variables|Default|SetHealth (- (Variables|Default|GetHealth) Damage)))
  (Development|PrintString (Utilities|String|ToString(Float) _output_get) true true "(R=1.000000,G=0.434760,B=0.000000,A=1.000000)" 5.0)
  (if (<= _output_get 0.0)
    (Development|PrintString "Dead" true true "(R=1.000000,G=0.000000,B=0.058791,A=1.000000)" 1e+01)
    (Variables|Default|SetAlive? false)
    ;[1 1 1] 物理シミュレーションでキャラクターが倒れる処理
    (Class|SkeletalMeshComponent|SetAllBodiesSimulatePhysics (Variables|Character|GetMesh) true)
    (Collision|SetCollisionEnabled (Variables|Character|GetMesh) "PhysicsOnly")
    ;[1 1 1] 当たり判定を削除
    (Components|DestroyComponent (Variables|Collision|GetCapsuleComponent))))

(fn ConstructionScript)