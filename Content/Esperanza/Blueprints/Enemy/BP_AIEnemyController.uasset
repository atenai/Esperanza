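; AI controller for enemies that runs the BT_AIEnemy behavior tree on BeginPlay.
; Its AI Perception component reacts only to the player character, setting the TargetActor blackboard key when the player is sensed and clearing it when lost.
; Both transitions print colored on-screen debug messages for detection and loss.
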(event OnTargetPerceptionUpdated(AIPerception)
  (params (Actor :type Actor%20Object%20Reference) (Stimulus :type AI%20Stimulus%20Structure))
  (if (== Actor (Game|GetPlayerCharacter 0))
    (if (.bSuccessfullySensed (Utilities|Struct|BreakAIStimulus Stimulus))
      (AI|Components|Blackboard|SetValueasObject (Variables|Default|GetBlackboard) (Utilities|Name|MakeLiteralName "TargetActor") Actor)
      (Development|PrintString "発見！！" true true "(R=1.000000,G=0.000000,B=0.279608,A=1.000000)")
      (else
        (AI|Components|Blackboard|SetValueasObject (Variables|Default|GetBlackboard) (Utilities|Name|MakeLiteralName "TargetActor") 0)
        (Development|PrintString "消失" true true "(R=0.078119,G=0.000000,B=1.000000,A=1.000000)")))))

(event EventBeginPlay
  (AI|RunBehaviorTree "/Game/Esperanza/Blueprints/Enemy/BT_AIEnemy.BT_AIEnemy") ; 使いたいビヘイビアツリーを選択する
)

(fn ConstructionScript)