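; Player character for a third-person rifle shooter, handling movement, HUD widgets, health and pickup effects.
; Timer-looped firing spends magazine ammo and applies point damage by line trace, from camera when aiming or muzzle otherwise, while timed reload refills from reserve.
; Aiming switches to a toggleable over-shoulder camera, slowing look speed and reddening the crosshair over Enemy-tagged actors.
; Lethal damage removes HUD, ragdolls the character and opens GameOver.
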(event Custom|On%20Fire
  (bind _weapon (Variables|Default|GetWeapon))
  (bind _returnvalue (Transformation|GetSocketTransform _weapon "MuzzleFlash" "RTS_World"))
  ;[1 1 1] 射撃アニメーションをループ再生
  (Animation|Montage|PlayMontage (Variables|Character|GetMesh) "/Game/Esperanza/Animations/MM_Rifle_Fire_Montage.MM_Rifle_Fire_Montage" ; 射撃アニメーションを再生
    (:then
      ;[1 1 1] マガジンの残弾数によって射撃できるか？どうかを分岐させる
      (if (< 0 (Variables|Default|Get現在のマガジン弾数))
        (Variables|Default|Set現在のマガジン弾数 (- (Variables|Default|Get現在のマガジン弾数) 1))
        (Effects|SpawnEmitteratLocation "/Game/MilitaryWeapSilver/FX/P_AssaultRifle_MuzzleFlash.P_AssaultRifle_MuzzleFlash" (.location _returnvalue) (.rotation _returnvalue)) ; マズルフラッシュのエフェクトを出す
        (Audio|PlaySoundatLocation "/Game/MilitaryWeapSilver/Sound/Rifle/Cues/RifleA_Fire_Cue.RifleA_Fire_Cue" (.location _returnvalue) "0, 0, 0" 1.0 1.0 0.0 0 0 0 0) ; 銃声音を再生する
        (if (Variables|Default|GetisAim) ; エイム中かどうか？
          (CallFunction|CameraRayFire)
          (else
            (CallFunction|GunRayFire)))
        (else
          ;[1 1 1] 射撃アニメーションのループ再生を終了させる
          (Utilities|Time|ClearandInvalidateTimerbyHandle (Variables|Default|GetFireTimer)))))))

(event Custom|回復薬
  (Variables|Default|SetHP (+ (Variables|Default|GetHP) 5e+01)))

(event Custom|弾薬箱
  (Variables|Default|Set残りの弾薬数 (+ (Variables|Default|Get残りの弾薬数) 60)))

(event EventBeginPlay
  (CallFunction|カメラの上下範囲の設定)
  ;[1 1 1] クロスヘアUIを作成する
  (bind _returnvalue (UserInterface|CreateWidget "/Game/Esperanza/UI/WBP_Crosshair.WBP_Crosshair_C"))
  (Variables|Default|SetCrosshairWidget _returnvalue)
  ;[1 1 1] プレイヤーHPゲージを作成する
  (bind _returnvalue_2 (UserInterface|CreateWidget "/Game/Esperanza/UI/WBP_PlayerHPGauge.WBP_PlayerHPGauge_C"))
  (bind _output_get (Variables|Default|SetHPBar _returnvalue_2))
  (UserInterface|Viewport|AddtoViewport _output_get 0)
  ;[1 1 1] マガジンのUIを作成
  (bind _returnvalue_3 (UserInterface|CreateWidget "/Game/Esperanza/UI/WBP_Magazine.WBP_Magazine_C"))
  (bind _output_get_2 (Variables|Default|SetMagazineUI _returnvalue_3))
  (UserInterface|Viewport|AddtoViewport _output_get_2 0)
  (CallFunction|InitReload))

(event EventTick
  (params (DeltaSeconds :type Float%20%28single-precision%29))
  (CallFunction|敵を捕らえたらカメラスピードを遅くする (Variables|Default|GetisAim))
  (Default|UpdateHealthBar (Variables|Default|GetHPBar) (/ (Variables|Default|GetHP) (Variables|Default|GetMaxHP))))

(event Game|Damage|EventPointDamage
  (params (Damage :type Float%20%28single-precision%29) (DamageType :type Damage%20Type%20Object%20Reference) (HitLocation :type Vector :default "0, 0, 0") (HitNormal :type Vector :default "0, 0, 0") (HitComponent :type Primitive%20Component%20Object%20Reference) (BoneName :type Name :default "None") (ShotFromDirection :type Vector :default "0, 0, 0") (InstigatedBy :type Controller%20Object%20Reference) (DamageCauser :type Actor%20Object%20Reference) (HitInfo :type Hit%20Result%20Structure%20%28by%20ref%29))
  (bind _死んだか_ (CallFunction|ダメージ処理 Damage))
  (if _死んだか_
    (Development|PrintString "Dead" true true "(R=1.000000,G=0.000000,B=0.058791,A=1.000000)" 1e+01)
    (CallFunction|UIDelete)
    (CallFunction|Death)
    ;[1 1 1] 数秒後にゲームオーバー画面に遷移する
    (Utilities|FlowControl|Delay 2.0)
    (Game|OpenLevel(byObjectReference) "/Game/Esperanza/Maps/GameOver.GameOver")))

(event Input|ActionEvents|InputActionFire
  (params (Key :type Key%20Structure :default "None"))
  (bind _weapon (Variables|Default|GetWeapon))
  (bind _returnvalue (Transformation|GetSocketTransform _weapon "MuzzleFlash" "RTS_World"))
  (:Pressed
    ;[1 1 1] 射撃アニメーションをループ再生
    (Animation|Montage|PlayMontage (Variables|Character|GetMesh) "/Game/Esperanza/Animations/MM_Rifle_Fire_Montage.MM_Rifle_Fire_Montage" ; 射撃アニメーションを再生
      (:then
        (bind _returnvalue_2 (Utilities|Time|SetTimerbyEvent (delegate Custom|On%20Fire) 0.1 true)) ; 0.1秒後にEventが実行される
        (Variables|Default|SetFireTimer _returnvalue_2)
        ;[1 1 1] マガジンの残弾数によって射撃できるか？どうかを分岐させる
        (if (< 0 (Variables|Default|Get現在のマガジン弾数))
          (Variables|Default|Set現在のマガジン弾数 (- (Variables|Default|Get現在のマガジン弾数) 1))
          (Effects|SpawnEmitteratLocation "/Game/MilitaryWeapSilver/FX/P_AssaultRifle_MuzzleFlash.P_AssaultRifle_MuzzleFlash" (.location _returnvalue) (.rotation _returnvalue)) ; マズルフラッシュのエフェクトを出す
          (Audio|PlaySoundatLocation "/Game/MilitaryWeapSilver/Sound/Rifle/Cues/RifleA_Fire_Cue.RifleA_Fire_Cue" (.location _returnvalue) "0, 0, 0" 1.0 1.0 0.0 0 0 0 0) ; 銃声音を再生する
          (if (Variables|Default|GetisAim) ; エイム中かどうか？
            (CallFunction|CameraRayFire)
            (else
              (CallFunction|GunRayFire)))
          (else
            ;[1 1 1] 射撃アニメーションのループ再生を終了させる
            (Utilities|Time|ClearandInvalidateTimerbyHandle (Variables|Default|GetFireTimer)))))))
  (:Released
    ;[1 1 1] 射撃アニメーションのループ再生を終了させる
    (Utilities|Time|ClearandInvalidateTimerbyHandle (Variables|Default|GetFireTimer))))

(event Input|ActionEvents|InputActionAiming
  (params (Key :type Key%20Structure :default "None"))
  (bind _mesh (Variables|Character|GetMesh))
  (bind _crosshairwidget (Variables|Default|GetCrosshairWidget))
  (bind _returnvalue (Components|SkeletalMesh|GetAnimInstance _mesh))
  (:Pressed
    (Variables|Default|SetisAim true) ; エイムしている
    (bind _asabp_character (Utilities|Casting|CastToABP_Character _returnvalue)) ; ABP_Characterにアクセスするためのノード
    (Variables|/Game/Esperanza/Animations/ABP_Character.ABP_Character_C|SetIsAiming? _asabp_character true) ; エイム用のアニメーションをON
    ;[1 1 1] 新しい肩越しカメラシステム
    (if (Variables|Default|GetCrosshairViewpoint)
      (CallFunction|SetViewpoint "300.000000,50.000000,70.000000" "0, 0, 0" false true) ; 右肩越しカメラ（Xが奥、Yが横、Zが縦）
      ;[1 1 1] クロスヘアを表示
      (UserInterface|Viewport|AddtoViewport _crosshairwidget 0)
      (else
        (CallFunction|SetViewpoint "300.000000,-50.000000,70.000000" "0, 0, 0" false true) ; 左肩越しカメラ（Xが奥、Yが横、Zが縦）
        (UserInterface|Viewport|AddtoViewport _crosshairwidget 0))))
  (:Released
    (Variables|Default|SetisAim false) ; エイムしていない
    (bind _asabp_character_2 (Utilities|Casting|CastToABP_Character _returnvalue))
    (Variables|/Game/Esperanza/Animations/ABP_Character.ABP_Character_C|SetIsAiming? _asabp_character_2 false) ; エイム用のアニメーションをOFF
    (CallFunction|SetViewpoint "0, 0, 0" "0, 0, 0" true false) ; 通常カメラ
    ;[1 1 1] クロスヘアを削除
    (Widget|RemovefromParent (Variables|Default|GetCrosshairWidget))))

(event Input|ActionEvents|InputActionToggleViewPoint
  (params (Key :type Key%20Structure :default "None"))
  (:Pressed
    (CallFunction|SetToggleViewPoint)))

(event Input|ActionEvents|InputActionReload
  (params (Key :type Key%20Structure :default "None"))
  (:Pressed
    (bind _isreload (CallFunction|リロードを許可するか？))
    (if _isreload
      (if (not (Variables|Default|GetisReloading)) ; リロード中か？
        (Variables|Default|SetisReloading true)
        (bind _returnvalue (Utilities|Time|SetTimerbyEvent (EventDispatchers|CreateEvent :!event SetReloadParcent) (Utilities|Time|GetWorldDeltaSeconds) true))
        (Variables|Default|SetreloadTimer _returnvalue)
        ;[1 1 1] リロード音を再生する
        (Audio|PlaySoundatLocation "/Game/Esperanza/Sound/Reload.Reload" (.location (Transformation|GetSocketTransform (Variables|Default|GetWeapon) "Clip_Bone" "RTS_World")) "0, 0, 0" 1.0 1.0 0.0 0 0 0 0) ; リロード音を再生する
        (Utilities|FlowControl|Delay 1.0)
        (CallFunction|Reload)))))

(event Input|AxisEvents|InputAxisTurn
  (params (AxisValue :type Float%20%28single-precision%29))
  ;[1 1 1] カメラ
  (Pawn|Input|AddControllerYawInput (* AxisValue (Variables|Default|GetcameraSpeed))))

(event Input|AxisEvents|InputAxisLookUp
  (params (AxisValue :type Float%20%28single-precision%29))
  ;[1 1 1] カメラ
  (Pawn|Input|AddControllerPitchInput (* AxisValue (Variables|Default|GetcameraSpeed))))

(event Input|AxisEvents|InputAxisMoveForward
  (params (AxisValue :type Float%20%28single-precision%29))
  ;[1 1 1] 移動
  (Pawn|Input|AddMovementInput (Math|Vector|GetForwardVector (Math|Rotator|MakeRotator 0.0 0.0 (.Yaw (Math|Rotator|BreakRotator (Pawn|GetControlRotation :!class /Script/Engine.Pawn))))) AxisValue false))

(event Input|AxisEvents|InputAxisMoveRight
  (params (AxisValue :type Float%20%28single-precision%29))
  ;[1 1 1] 移動
  (Pawn|Input|AddMovementInput (Math|Vector|GetRightVector (Math|Rotator|MakeRotator 0.0 0.0 (.Yaw (Math|Rotator|BreakRotator (Pawn|GetControlRotation :!class /Script/Engine.Pawn))))) AxisValue false))

(fn ConstructionScript)

(fn SetViewpoint
  (params (NewLocation :type Vector) (NewRotation :type Rotator) (Orient%20Rotation%20to%20Movement :type Boolean) (Use%20Controller%20Rotation%20Yaw :type Boolean))
  (Transformation|SetRelativeLocationAndRotation (Variables|Default|GetCamera) NewLocation NewRotation false false)
  (Variables|/Script/Engine.CharacterMovementComponent|SetbOrientRotationToMovement (Variables|Character|GetCharacterMovement) Orient%20Rotation%20to%20Movement)
  (Variables|Default|SetbUseControllerRotationYaw Use%20Controller%20Rotation%20Yaw))

(fn SetToggleViewPoint
  (if (Variables|Default|GetCrosshairViewpoint)
    (Variables|Default|SetCrosshairViewpoint false) ; 肩越し左肩視点カメラ
    (else
      (Variables|Default|SetCrosshairViewpoint true) ; 肩越し右肩視点カメラ
    ))
  (Development|PrintString (Utilities|String|ToString(Boolean) (Variables|Default|GetCrosshairViewpoint)) true true "(R=1.000000,G=0.000000,B=0.028928,A=1.000000)" 1e+01))

(fn ダメージ処理
  (params (ダメージ数 :type Float%20%28double-precision%29))
  ;[1 1 1] ダメージを受ける処理
  (CameraShakes|StartCameraShake (Game|GetPlayerCameraManager 0) "/Game/Esperanza/Blueprints/Player/BP_DamageCameraShake.BP_DamageCameraShake_C" 1.0 "CameraLocal" "0, 0, 0")
  (bind _output_get (Variables|Default|SetHP (- (Variables|Default|GetHP) ダメージ数)))
  (return (<= _output_get 0.0)))

(fn UIDelete
  ;[1 1 1] 2層式HPゲージのUIを消す、そうしないとプレイヤーキャラクターが見つけられずエラーになる
  (Widget|RemovefromParent (Variables|Default|GetHPBar))
  ;[1 1 1] マガジンUIを消す
  (Widget|RemovefromParent (Variables|Default|GetMagazineUI)))

(fn Death
  ;[1 1 1] 物理シミュレーションでキャラクターが倒れる処理
  (Class|SkeletalMeshComponent|SetAllBodiesSimulatePhysics (Variables|Character|GetMesh) true)
  (Collision|SetCollisionEnabled (Variables|Character|GetMesh) "PhysicsOnly")
  (Input|DisableInput (Game|GetPlayerController 0)) ; キャラクターの入力を受け付けなくするノード
)

(fn GunRayFire
  (bind _weapon (Variables|Default|GetWeapon))
  (bind _returnvalue (Transformation|GetSocketTransform _weapon "MuzzleFlash" "RTS_World"))
  ;[1 1 1 1 30] 銃口からレイを出して攻撃する
  (bind (_outhit _returnvalue_2) (Collision|LineTraceByChannel (.location _returnvalue) (+ (.location _returnvalue) (* (Math|Vector|GetForwardVector (.rotation _returnvalue)) 5e+03)) "TraceTypeQuery2" false 0 "ForDuration" true "(R=0.000000,G=1.000000,B=0.700000,A=1.000000)")) ; StartからEndに向かってレイを飛ばすノード
  (Game|SpawnActorfromClass "/Game/Esperanza/Blueprints/Player/BP_RilfeTracer.BP_RilfeTracer_C" (Transformation|GetSocketTransform (Variables|Default|GetWeapon) "MuzzleFlash" "RTS_World") "AlwaysSpawn" "OverrideRootScale" 0 0) ; 銃弾の軌跡のアクターを生成する
  (if _returnvalue_2
    (Game|Damage|ApplyPointDamage (.HitActor (Collision|BreakHitResult _outhit)) 1e+01 (.TraceStart (Collision|BreakHitResult _outhit)) _outhit) ; アクターにダメージを与えるノード
  ))

(fn CameraRayFire
  (bind _camera (Variables|Default|GetCamera))
  (bind _weapon (Variables|Default|GetWeapon))
  (bind _returnvalue (Transformation|GetSocketTransform _weapon "MuzzleFlash" "RTS_World"))
  (bind _returnvalue_2 (Transformation|GetWorldLocation _camera))
  ;[1 1 1 1 30] カメラからレイを出して攻撃する
  (bind (_outhit _returnvalue_3) (Collision|LineTraceByChannel _returnvalue_2 (+ _returnvalue_2 (* (Math|Vector|GetForwardVector (Transformation|GetWorldRotation (Variables|Default|GetCamera))) 5e+03)) "TraceTypeQuery2" false 0 "ForDuration" true "(R=1.000000,G=0.000000,B=0.039356,A=1.000000)" "(R=1.000000,G=0.000000,B=1.000000,A=1.000000)")) ; StartからEndに向かってレイを飛ばすノード
  (Game|SpawnActorfromClass "/Game/Esperanza/Blueprints/Player/BP_RilfeTracer.BP_RilfeTracer_C" (Math|Transform|MakeTransform (.location _returnvalue) (Math|Rotator|FindLookatRotation (.location _returnvalue) (.TraceEnd (Collision|BreakHitResult _outhit))) (.scale _returnvalue)) "AlwaysSpawn" "OverrideRootScale" 0 0) ; 銃弾の軌跡のアクターを生成する
  (if _returnvalue_3
    (Game|Damage|ApplyPointDamage (.HitActor (Collision|BreakHitResult _outhit)) 1e+01 (.TraceStart (Collision|BreakHitResult _outhit)) _outhit) ; アクターにダメージを与えるノード
  ))

(fn Reload
  (bind _initammo (Variables|Default|GetinitAmmo))
  (Utilities|Time|ClearandInvalidateTimerbyHandle (Variables|Default|GetreloadTimer))
  ;[1 1 1] マガジンを給弾する処理
  (LocalVariables|SettempCurrentAmmo (Variables|Default|Get現在のマガジン弾数))
  (Variables|Default|Set現在のマガジン弾数 (Math|Integer|SelectInt (+ (Variables|Default|Get残りの弾薬数) (Variables|Default|Get現在のマガジン弾数)) _initammo (< (+ (Variables|Default|Get残りの弾薬数) (Variables|Default|Get現在のマガジン弾数)) _initammo)))
  ;[1 1 1] 残りの弾数を計算する処理
  (Variables|Default|Set残りの弾薬数 (Math|Integer|Max(Integer) (- (Variables|Default|Get残りの弾薬数) (- (Variables|Default|GetinitAmmo) (LocalVariables|GettempCurrentAmmo)))))
  (bind _output_get (Variables|Default|SetreloadProgressTimer 0.0))
  (Default|SetPercent (Variables|Default|GetreloadUIRef) _output_get)
  (Variables|Default|SetisReloading false))

(fn SetReloadParcent
  (bind _output_get (Variables|Default|SetreloadProgressTimer (+ (Variables|Default|GetreloadProgressTimer) (Utilities|Time|GetWorldDeltaSeconds))))
  (Default|SetPercent (Variables|Default|GetreloadUIRef) _output_get))

(fn InitReload
  ;[1 1 1] リロードUIを作成
  (bind _returnvalue (UserInterface|CreateWidget "/Game/Esperanza/UI/WBP_ReloadUI.WBP_ReloadUI_C"))
  (bind _output_get (Variables|Default|SetreloadUIRef _returnvalue))
  (UserInterface|Viewport|AddtoViewport _output_get 0)
  (Variables|Default|Set現在のマガジン弾数 (Variables|Default|GetinitAmmo))
  (Variables|Default|Set残りの弾薬数 (* (Variables|Default|GetinitAmmo) (Variables|Default|GetmagazineSize)))
  (Variables|Default|SetisReloading false))

(fn DebugAmmo
  (Development|PrintString (Utilities|String|Append "Current : " (Utilities|String|ToString(Integer) (Variables|Default|Get現在のマガジン弾数)) " 
" "Max : " (Utilities|String|ToString(Integer) (Variables|Default|Get残りの弾薬数))) true true "(R=0.000000,G=0.660000,B=1.000000,A=1.000000)" 0.0))

(fn リロードを許可するか？
  ;[1 1 1] リロードを許可するか？
  (return (and (!= (Variables|Default|GetinitAmmo) (Variables|Default|Get現在のマガジン弾数)) (< 0 (Variables|Default|Get残りの弾薬数)))))

(fn カメラの上下範囲の設定
  (bind _returnvalue (Game|GetPlayerCameraManager 0))
  (Variables|/Script/Engine.PlayerCameraManager|SetViewPitchMax _returnvalue 1e+01)
  (Variables|/Script/Engine.PlayerCameraManager|SetViewPitchMin _returnvalue -7e+01))

(fn 敵を捕らえたらカメラスピードを遅くする
  (params (isAim :type Boolean))
  (bind _camera (Variables|Default|GetCamera))
  (bind _returnvalue (Transformation|GetWorldLocation _camera))
  (if isAim ; エイムしているか？
    (bind (_outhit _returnvalue_2) (Collision|LineTraceByChannel _returnvalue (+ _returnvalue (* (Math|Vector|GetForwardVector (Transformation|GetWorldRotation (Variables|Default|GetCamera))) 1e+04)) "TraceTypeQuery2" false 0 "None" true "(R=1.000000,G=0.000000,B=0.039356,A=1.000000)")) ; StartからEndに向かってレイを飛ばすノード
    (if _returnvalue_2 ; レイが何かにヒットしたか？
      (if (Actor|ActorHasTag (.HitActor (Collision|BreakHitResult _outhit)) "Enemy") ; ヒットした物はエネミーか？
        (Variables|Default|SetcameraSpeed 0.1)
        (Default|赤色に変える (Variables|Default|GetCrosshairWidget))
        (else
          (Variables|Default|SetcameraSpeed 1.0)
          (Default|白色に変える (Variables|Default|GetCrosshairWidget))))
      (else
        (Variables|Default|SetcameraSpeed 1.0)
        (Default|白色に変える (Variables|Default|GetCrosshairWidget))))
    (else
      (Variables|Default|SetcameraSpeed 1.0)
      (Default|白色に変える (Variables|Default|GetCrosshairWidget)))))